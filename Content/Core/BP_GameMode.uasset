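; Game mode that runs the level loop, alternating randomly picked combat arenas with a shop and offering a separately triggered treasure room.
; Rooms stream in as level instances, with each arena 4000 units below the last, and OnLevelShown teleports the player to the spawn point.
; Arenas start their BP_AISpawner, and SpawnerEnded advances the loop.
; MusicManager handles track changes and light/mesh deregistration; leaving the shop adds brief slow motion.
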(event Custom|SpawnTreasureRoom
  (bind _musicmanager (Variables|Default|GetMusicManager))
  ;[1 1 1] Shop Spawning
  (Class|AMusicManager|DeRegisterLights _musicmanager)
  (Class|AMusicManager|DeRegisterMeshes _musicmanager)
  (Utilities|IsValid (Variables|Streaming|GetTreasureLevelAsset)
    (:Is%20Valid
      (Variables|/Script/Engine.LevelStreaming|SetbShouldBeVisible (Variables|Streaming|GetTreasureLevelAsset) false)
      (Variables|/Script/Engine.LevelStreaming|SetbShouldBeLoaded (Variables|Streaming|GetTreasureLevelAsset) false))
    (:Is%20Not%20Valid
      _))
  (bind _returnvalue (Class|LevelStreamingDynamic|LoadLevelInstance (Variables|Streaming|GetTreasureLevel) (Math|Vector|MakeVector -1e+03 -1e+03 4e+03) "0, 0, 0"))
  (Variables|Streaming|SetTreasureLevelAsset _returnvalue)
  (EventDispatchers|AssignOnLevelShown _returnvalue (delegate Custom|TransferToTreasureRoom)))

(event Custom|SpawnerEnded
  ;[1 1 1] Spawners
  (CallFunction|SpawnArena))

(event Custom|TransferToTreasureRoom
  ;[1 1 1] Shop Spawning
  (bind _spawnlocation (Class|RogueLikeMusicGameGameMode|GetSpawnLocationinLevel (Class|LevelStreaming|GetLoadedLevel (Variables|Streaming|GetTreasureLevelAsset))))
  (Transformation|SetActorLocation (Game|GetPlayerCharacter 0) _spawnlocation false true))

(event Custom|StartSpawner
  ;[1 1 1] Spawners
  (bind _returnvalue (Class|RogueLikeMusicGameGameMode|GetAISpawnerinLevel (Class|LevelStreaming|GetLoadedLevel (Variables|Streaming|GetLoadedLevelAsset))))
  (bind _asbp_aispawner (Utilities|Casting|CastToBP_AISpawner _returnvalue))
  (Default|StartSpawning _asbp_aispawner))

(event Custom|SpawnArena
  (bind _currentlevel (Variables|Default|GetCurrentLevel))
  (bind _musicmanager (Variables|Default|GetMusicManager))
  (bind _levels (Variables|Streaming|GetLevels))
  ;[1 1 1] Arena Spawning
  (Math|Integer|IncrementInt _currentlevel
    (:%20%20
      (Math|Integer|IncrementInt (Variables|Default|GetAccumulatedLevels)
        (:%20%20
          (if (>= _currentlevel 2)
            (CallFunction|SpawnShop)
            (else
              (Class|AMusicManager|DeRegisterLights _musicmanager)
              (Class|AMusicManager|DeRegisterMeshes _musicmanager)
              (bind _output_get (Variables|Streaming|SetZ (- (Variables|Streaming|GetZ) 4e+03)))
              (bind _returnvalue (Class|LevelStreamingDynamic|LoadLevelInstance (Utilities|Array|Get(acopy) _levels (Math|Random|RandomInteger (Utilities|Array|Length _levels))) (Math|Vector|MakeVector 0.0 0.0 _output_get) "0, 0, 0"))
              (Variables|Streaming|SetOldLevelAsset (Variables|Streaming|GetLoadedLevelAsset))
              (bind _output_get_2 (Variables|Streaming|SetLoadedLevelAsset _returnvalue))
              (EventDispatchers|AssignOnLevelShown _output_get_2 (delegate Custom|Transfer)))))))))

(event Custom|Transfer
  (bind _oldlevelasset (Variables|Streaming|GetOldLevelAsset))
  ;[1 1 1] Arena Spawning
  (Utilities|IsValid _oldlevelasset
    (:Is%20Valid
      (Variables|/Script/Engine.LevelStreaming|SetbShouldBeVisible _oldlevelasset false)
      (Variables|/Script/Engine.LevelStreaming|SetbShouldBeLoaded _oldlevelasset false))
    (:Is%20Not%20Valid
      _))
  (bind _spawnlocation (Class|RogueLikeMusicGameGameMode|GetSpawnLocationinLevel (Class|LevelStreaming|GetLoadedLevel (Variables|Streaming|GetLoadedLevelAsset))))
  (Transformation|SetActorLocation (Game|GetPlayerCharacter 0) _spawnlocation false true)
  (CallFunction|StartSpawner)
  (Variables|Default|SetbIsShopLocked false))

(event Custom|EndShop
  (if (not (Variables|Default|GetbIsShopLocked))
    (Variables|Default|SetbIsShopLocked true)
    (Class|AMusicManager|SetNewTrack (Variables|Default|GetMusicManager))
    (Utilities|Time|SetGlobalTimeDilation 0.1)
    (Utilities|FlowControl|Delay 0.25)
    (Variables|Default|SetCurrentLevel 0)
    (CallFunction|SpawnArena)
    (Utilities|Time|SetGlobalTimeDilation 1.0)))

(event Custom|SpawnShop
  (bind _musicmanager (Variables|Default|GetMusicManager))
  ;[1 1 1] Shop Spawning
  (Class|AMusicManager|StartShopTrack (Variables|Default|GetMusicManager))
  (Class|AMusicManager|DeRegisterLights _musicmanager)
  (Class|AMusicManager|DeRegisterMeshes _musicmanager)
  (Utilities|IsValid (Variables|Streaming|GetShopLevelAsset)
    (:Is%20Valid
      (Variables|/Script/Engine.LevelStreaming|SetbShouldBeVisible (Variables|Streaming|GetShopLevelAsset) false)
      (Variables|/Script/Engine.LevelStreaming|SetbShouldBeLoaded (Variables|Streaming|GetShopLevelAsset) false))
    (:Is%20Not%20Valid
      _))
  (bind _returnvalue (Class|LevelStreamingDynamic|LoadLevelInstance (Variables|Streaming|GetShopLevel) (Math|Vector|MakeVector 1e+03 1e+03 4e+03) "0, 0, 0"))
  (Variables|Streaming|SetShopLevelAsset _returnvalue)
  (EventDispatchers|AssignOnLevelShown _returnvalue (delegate Custom|TransferToShop)))

(event Custom|TransferToShop
  ;[1 1 1] Shop Spawning
  (bind _spawnlocation (Class|RogueLikeMusicGameGameMode|GetSpawnLocationinLevel (Class|LevelStreaming|GetLoadedLevel (Variables|Streaming|GetShopLevelAsset))))
  (Transformation|SetActorLocation (Game|GetPlayerCharacter 0) _spawnlocation false true))

(fn ConstructionScript)