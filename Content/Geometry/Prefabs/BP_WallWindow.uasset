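; BP_WallWindow is a geometry prefab, named as a wall section with a window, that groups twelve static mesh components into one actor.
; Its only logic is GetStaticMeshes, which returns those components as a hand-ordered array.
; The construction script is empty and the BeginPlay, overlap and Tick events are unused stubs.
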(event EventBeginPlay)

(event Collision|EventActorBeginOverlap
  (params (OtherActor :type Actor%20Object%20Reference)))

(event EventTick
  (params (DeltaSeconds :type Float%20%28single-precision%29)))

(fn ConstructionScript)

(fn GetStaticMeshes
  (return (Utilities|Array|MakeArray (Variables|Default|GetStaticMeshComponent6) (Variables|Default|GetStaticMeshComponent1) (Variables|Default|GetStaticMeshComponent2) (Variables|Default|GetStaticMeshComponent3) (Variables|Default|GetStaticMeshComponent4) (Variables|Default|GetStaticMeshComponent5) (Variables|Default|GetStaticMeshComponent0) (Variables|Default|GetStaticMeshComponent7) (Variables|Default|GetStaticMeshComponent8) (Variables|Default|GetStaticMeshComponent9) (Variables|Default|GetStaticMeshComponent10) (Variables|Default|GetStaticMeshComponent11))))