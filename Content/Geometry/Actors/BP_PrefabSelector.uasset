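; BP_PrefabSelector is a placeholder actor that swaps in a random prefab with randomized materials at BeginPlay.
; It spawns a random class from Actors at its own transform, then gets that actor's static meshes through a GetStaticMeshes message.
; Each mesh receives a random pick from Materials on slot 0.
; DestroyActor on the selector sits inside that loop, so it remains if no meshes return.
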(event EventBeginPlay
  (bind _actors (Variables|Default|GetActors))
  (bind _returnvalue (Game|SpawnActorfromClass (Utilities|Array|Get(acopy) _actors (Math|Random|RandomInteger (Utilities|Array|Length _actors))) (Transformation|GetActorTransform) "Undefined" self 0))
  (bind _newparam (Class|BPIInterface|GetStaticMeshes(Message) _returnvalue))
  (if (> (Utilities|Array|Length _newparam) 0)
    (for _array_element _newparam
      (bind _randnum (CallFunction|RandomNumMat))
      (Rendering|Material|SetMaterial _array_element 0 (Utilities|Array|Get(acopy) (Variables|Default|GetMaterials) _randnum))
      (Actor|DestroyActor))))

(fn ConstructionScript)

(fn RandomNumMat
  (bind _output_get (Variables|Default|SetVisibleNum (Math|Random|RandomIntegerinRange 0 (- (Utilities|Array|Length (Variables|Default|GetMaterials)) 1))))
  (return _output_get))