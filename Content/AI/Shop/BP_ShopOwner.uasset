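; Shop owner actor with a hidden head bone that pulses to the music and ends the shop when damaged.
; On begin play it retries every half second until it gets the music manager from the game mode.
; Each tick it maps the first returned spectrum value to the mesh's X and Y scale.
; Any damage calls EndShop on the game mode, then ragdolls the mesh with a pelvis impulse away from the player.
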(event EventBeginPlay
  (Components|SkinnedMesh|HideBonebyName (Variables|Default|GetSkeletalMesh) "head" "PBO_None")
  (bind _asbp_game_mode (Utilities|Casting|CastToBP_GameMode (Game|GetGameMode) :!label _label)
    (:then
      (bind _asbp_music_manager (Utilities|Casting|CastToBP_MusicManager (Variables|/Script/RogueLikeMusicGame.RogueLikeMusicGameGameMode|GetMusicManager _asbp_game_mode))
        (:then
          (Variables|Default|SetMusicManager _asbp_music_manager))
        (:CastFailed
          (Utilities|FlowControl|Delay 0.5 :!label _label_2)
          (goto _label))))
    (:CastFailed
      (goto _label_2))))

(event Collision|EventActorBeginOverlap
  (params (OtherActor :type Actor%20Object%20Reference)))

(event EventTick
  (params (DeltaSeconds :type Float%20%28single-precision%29))
  (bind _outspectrum (Default|GetSpectrumArray (Variables|Default|GetMusicManager) 1))
  (Transformation|SetWorldScale3D (Variables|Default|GetSkeletalMesh) (Math|Vector|MakeVector (Math|Float|MapRangeClamped (Math|Float|Absolute(Float) (Utilities|Array|Get(acopy) _outspectrum)) 0.0 3e+01 1.0 2.0) (Math|Float|MapRangeClamped (Math|Float|Absolute(Float) (Utilities|Array|Get(acopy) _outspectrum)) 0.0 3e+01 1.0 2.0) 1.0)))

(event Game|Damage|EventAnyDamage
  (params (Damage :type Float%20%28single-precision%29) (DamageType :type Damage%20Type%20Object%20Reference) (InstigatedBy :type Controller%20Object%20Reference) (DamageCauser :type Actor%20Object%20Reference))
  (bind _skeletalmesh (Variables|Default|GetSkeletalMesh))
  (bind _asbp_game_mode (Utilities|Casting|CastToBP_GameMode (Game|GetGameMode)))
  (Default|EndShop _asbp_game_mode)
  (Class|SkeletalMeshComponent|SetAllBodiesSimulatePhysics _skeletalmesh true)
  (Collision|SetCollisionEnabled _skeletalmesh "QueryAndPhysics")
  (Physics|AddImpulse _skeletalmesh (* (Math|Vector|Normalize (- (Transformation|GetActorLocation) (Transformation|GetActorLocation (Game|GetPlayerCharacter 0)))) 5e+01) "pelvis" false))

(fn ConstructionScript)