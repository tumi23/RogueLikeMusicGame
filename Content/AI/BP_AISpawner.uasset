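; AI spawner for a roguelike music game that accumulates a spawn counter from the music, though the spawning itself is not implemented yet.
; On BeginPlay it picks a random wave row from a data table, caches the music manager and registers with the game mode.
; Between Start and End, each Tick adds a music waveform sample to the counter, but reaching the limit triggers nothing.
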(event Custom|Start
  (Variables|Default|SetStarted true))

(event Custom|End
  (Variables|Default|SetStarted false))

(event EventBeginPlay
  (bind _outrownames (DataTable|GetDataTableRowNames (Variables|Default|GetDataTable)))
  (bind _returnvalue (Utilities|GetDataTableRow (Variables|Default|GetDataTable) (Utilities|Array|Get(acopy) _outrownames (Math|Random|RandomInteger (- (Utilities|Array|Length _outrownames) 1))))
    (:then
      (Variables|Default|SetWaveToUse _returnvalue))
    (:RowNotFound
      _))
  (bind _asrogue_like_music_game_game_mode (Utilities|Casting|CastToRogueLikeMusicGameGameMode (Game|GetGameMode))
    (:then
      (Variables|Default|SetGameMode _asrogue_like_music_game_game_mode))
    (:CastFailed
      _))
  (bind _asbp_music_manager (Utilities|Casting|CastToBP_MusicManager (Variables|/Script/RogueLikeMusicGame.RogueLikeMusicGameGameMode|GetMusicManager (Variables|Default|GetGameMode))))
  (Variables|Default|SetMusicManager _asbp_music_manager)
  (bind _asbp_game_mode (Utilities|Casting|CastToBP_GameMode _asrogue_like_music_game_game_mode))
  (Default|RegisterSpawner _asbp_game_mode self))

(event EventTick
  (params (DeltaSeconds :type Float%20%28single-precision%29))
  (if (Variables|Default|GetStarted)
    (bind _outspectrum (Default|GetMusicWaveform (Variables|Default|GetMusicManager) 1))
    (bind _output_get (Variables|Default|SetSpawnCounter (+ (Variables|Default|GetSpawnCounter) (Utilities|Array|Get(acopy) _outspectrum))))
    (if (>= _output_get (Variables|Default|GetSpawnUpperLimit))
      _)))

(fn ConstructionScript)