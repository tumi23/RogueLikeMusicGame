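; Base enemy AI character that shoots at the player and handles its own damage and death.
; Fire spawns a projectile rotated toward player zero's character.
; Damage drains Health; the first lethal hit broadcasts OnKilled, awards BroCoins and score to the player, and stops the AI controller's brain logic.
; The mesh then ragdolls, breaking constraints at every socket name with an impulse away from the player, before a delayed destroy.
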(event Custom|Fire
  (Game|SpawnActorfromClass "/Game/AI/Enemy/BP_BaseProjectile.BP_BaseProjectile_C" (Math|Transform|MakeTransform (Transformation|GetActorLocation) (Math|Rotator|FindLookatRotation (Transformation|GetActorLocation) (Transformation|GetActorLocation (Game|GetPlayerCharacter 0)))) "Undefined" 0 0))

(event EventBeginPlay)

(event Collision|EventActorBeginOverlap
  (params (OtherActor :type Actor%20Object%20Reference)))

(event EventTick
  (params (DeltaSeconds :type Float%20%28single-precision%29)))

(event Game|Damage|EventAnyDamage
  (params (Damage :type Float%20%28single-precision%29) (DamageType :type Damage%20Type%20Object%20Reference) (InstigatedBy :type Controller%20Object%20Reference) (DamageCauser :type Actor%20Object%20Reference))
  (bind _mesh (Variables|Character|GetMesh))
  (bind _output_get (Variables|Default|SetHealth (- (Variables|Default|GetHealth) Damage)))
  (if (and (<= _output_get 0.0) (not (Variables|Default|GetIsDead)))
    (Default|CallOnKilled self)
    (Variables|Default|SetIsDead true)
    (bind _asfirst_person_character (Utilities|Casting|CastToFirstPersonCharacter (Game|GetPlayerCharacter 0)))
    (Variables|/Script/RogueLikeMusicGame.RogueLikeMusicGameCharacter|SetCurrentBroCoins _asfirst_person_character (+ (Variables|/Script/RogueLikeMusicGame.RogueLikeMusicGameCharacter|GetCurrentBroCoins _asfirst_person_character) 25))
    (Variables|/Script/RogueLikeMusicGame.RogueLikeMusicGameCharacter|SetTotalScore _asfirst_person_character (+ (Variables|/Script/RogueLikeMusicGame.RogueLikeMusicGameCharacter|GetTotalScore _asfirst_person_character) 25))
    (|KillController)
    (Collision|SetCollisionEnabled (Variables|Collision|GetCapsuleComponent) "NoCollision")
    (Collision|SetCollisionEnabled _mesh "PhysicsOnly")
    (Class|SkeletalMeshComponent|SetAllBodiesSimulatePhysics _mesh true)
    (for _array_element (Transformation|GetAllSocketNames _mesh)
      (Class|SkeletalMeshComponent|BreakConstraint _mesh (* (Math|Vector|Normalize (- (Transformation|GetActorLocation) (Transformation|GetActorLocation (Game|GetPlayerCharacter 0)))) 100) "0, 0, 0" _array_element))
    (Utilities|FlowControl|Delay 5.0)
    (Actor|DestroyActor)))

(fn ConstructionScript)