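; Level enemy spawner that picks a random data table row of waves and scales their counts by the game mode's accumulated levels.
; While started, Tick builds a spawn counter from music spectrum amplitude, spawning the front wave's enemies at random spawn points in sync with audio intensity.
; Death callbacks track living enemies and notify the game mode once all waves are cleared.
; The logic setting Started and manager references is unconnected.
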(event Custom|StartSpawning
  (bind _datatable (Variables|Default|GetDatatable))
  (bind _outrownames (DataTable|GetDataTableRowNames _datatable))
  (bind _returnvalue (Utilities|GetDataTableRow _datatable (Utilities|Array|Get(acopy) _outrownames (Math|Random|RandomInteger (- (Utilities|Array|Length _outrownames) 1))))
    (:then
      (bind _output_get (Variables|Default|SetWaves (Utilities|Struct|BreakWaves _returnvalue)))
      (bind _asbp_game_mode (Utilities|Casting|CastToBP_GameMode (Game|GetGameMode)))
      (for (_array_element _array_index) _output_get
        (bind _structout (Utilities|Struct|SetmembersinWaveInfo _array_element (Math|Float|Truncate (* (.Count (Utilities|Struct|BreakWaveInfo _array_element)) (* (Variables|/Game/Core/BP_GameMode.BP_GameMode_C|GetAccumulatedLevels _asbp_game_mode) 0.5)))))
        (Utilities|Array|SetArrayElem (Variables|Default|GetWaves) _array_index _structout)))))

(event Custom|EnemyDied
  (Variables|Default|SetEnemiesAlive (- (Variables|Default|GetEnemiesAlive) 1))
  (if (and (not (Variables|Default|GetStarted)) (<= (Variables|Default|GetEnemiesAlive) 0))
    (Default|SpawnerEnded (Variables|Default|GetGameMode))))

(event EventBeginPlay)

(event Collision|EventActorBeginOverlap
  (params (OtherActor :type Actor%20Object%20Reference)))

(event EventTick
  (params (DeltaSeconds :type Float%20%28single-precision%29))
  (bind _waves (Variables|Default|GetWaves))
  (bind _spawnpoints (Variables|Default|GetSpawnPoints))
  (bind _output (Utilities|Array|Get(acopy) _waves))
  (bind (_enemytype _count) (Utilities|Struct|BreakWaveInfo _output))
  (if (Variables|Default|GetStarted)
    (bind _outspectrum (Default|GetSpectrumArray (Variables|Default|GetMusicManager) 1))
    (bind _output_get (Variables|Default|SetSpawnCount (+ (* (Math|Float|Absolute(Float) (Utilities|Array|Get(acopy) _outspectrum)) DeltaSeconds) (Variables|Default|GetSpawnCount))))
    (if (>= _output_get (Variables|Default|GetSpawnRate))
      (Variables|Default|SetSpawnCount 0.0)
      (bind _returnvalue (Game|SpawnActorfromClass _enemytype (Math|Transform|MakeTransform (Transformation|GetActorLocation (Utilities|Array|Get(acopy) _spawnpoints (Math|Random|RandomInteger (Utilities|Array|Length _spawnpoints)))) "0, 0, 0" "1,1,1") "Undefined" 0 0))
      (EventDispatchers|BindEventtoOnKilled _returnvalue (delegate Custom|EnemyDied))
      (Variables|Default|SetEnemiesAlive (+ (Variables|Default|GetEnemiesAlive) 1))
      (bind _result (Math|Integer|DecrementInt _count)
        (:%20%20
          (bind _structout (Utilities|Struct|SetmembersinWaveInfo _output _result))
          (Utilities|Array|SetArrayElem _waves 0 _structout)
          (if (<= _result 0)
            (Utilities|Array|RemoveIndex _waves)
            (if (<= (Utilities|Array|Length (Variables|Default|GetWaves)) 0)
              (Variables|Default|SetStarted false))))))))

(fn ConstructionScript)